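; DamageBox is a test actor that damages the player character when it enters the box volume.
; BeginPlay caches the player as a MainCharacter_BP reference, and the Box overlap events react only to that character.
; Entering applies a fixed hit of damage through a DoOnce gate, which leaving the box resets, so damage lands once per entry rather than continuously.
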(event OnComponentBeginOverlap(Box)
  (params (OverlappedComponent :type Primitive%20Component%20Object%20Reference) (OtherActor :type Actor%20Object%20Reference) (OtherComp :type Primitive%20Component%20Object%20Reference) (OtherBodyIndex :type Integer) (bFromSweep :type Boolean) (SweepResult :type Hit%20Result%20Structure%20%28by%20ref%29))
  (if (== OtherActor (Variables|Default|GetCharacterRef))
    (Utilities|FlowControl|DoOnce false
      (:Completed
        (Game|Damage|ApplyDamage OtherActor 1.0 0 0)))))

(event OnComponentEndOverlap(Box)
  (params (OverlappedComponent :type Primitive%20Component%20Object%20Reference) (OtherActor :type Actor%20Object%20Reference) (OtherComp :type Primitive%20Component%20Object%20Reference) (OtherBodyIndex :type Integer))
  (if (== OtherActor (Variables|Default|GetCharacterRef))
    (Utilities|FlowControl|DoOnce false) ; enters at Reset
  ))

(event EventBeginPlay
  (bind _asmain_character_bp (Utilities|Casting|CastToMainCharacter_BP (Game|GetPlayerCharacter 0)))
  (Variables|Default|SetCharacterRef _asmain_character_bp))

(event Collision|EventActorBeginOverlap
  (params (OtherActor :type Actor%20Object%20Reference)))

(event EventTick
  (params (DeltaSeconds :type Float%20%28single-precision%29)))

(fn ConstructionScript)