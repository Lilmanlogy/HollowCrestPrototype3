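; Game Instance that owns the save system, persisting the player's health, stun and slow ammo, and collected relics.
; LoadGame stores the slot name and loads or creates the SaveGameOcject cached as SaveGameData.
; SavePlayerData copies MainCharacter_BP values into its struct and writes the slot; ClearSaveData deletes the slot.
; LoadPlayerData restores values from the cached object when the slot exists, ignoring its own fresh load result.
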(event Custom|Load%20Game
  (params (SaveSlot :type String))
  (bind _output_get (Variables|Default|SetSaveSlot SaveSlot))
  (bind _returnvalue (SaveGame|DoesSaveGameExist _output_get))
  (if _returnvalue
    (bind _returnvalue_2 (SaveGame|LoadGamefromSlot (Variables|Default|GetSaveSlot)))
    (bind _assave_game_ocject (Utilities|Casting|CastToSaveGameOcject _returnvalue_2))
    (Variables|Default|SetSaveGameData _assave_game_ocject)
    (else
      (bind _returnvalue_3 (SaveGame|CreateSaveGameObject "/Game/Blueprints/SaveSystem/SaveGameOcject.SaveGameOcject_C"))
      (Variables|Default|SetSaveGameData _returnvalue_3))))

(fn SavePlayerData
  (bind _asmain_character_bp (Utilities|Casting|CastToMainCharacter_BP (Game|GetPlayerCharacter 0)))
  (Variables|Default|SetPlayer%20Ref%20Save _asmain_character_bp)
  (Utilities|FlowControl|Sequence
    (:then_1
      (Variables|/Game/Blueprints/SaveSystem/SaveGameOcject.SaveGameOcject_C|SetPlayerSaveStruct (Variables|Default|GetSaveGameData) (Utilities|Struct|MakePlayerSaveStruct (Variables|/Game/Blueprints/MainCharacter_BP.MainCharacter_BP_C|GetHealth (Variables|Default|GetPlayer%20Ref%20Save)) (Variables|/Game/Blueprints/MainCharacter_BP.MainCharacter_BP_C|GetCurrentStunAmmo (Variables|Default|GetPlayer%20Ref%20Save)) (Variables|/Game/Blueprints/MainCharacter_BP.MainCharacter_BP_C|GetStun%20Ammo%20Reserve (Variables|Default|GetPlayer%20Ref%20Save)) (Variables|/Game/Blueprints/MainCharacter_BP.MainCharacter_BP_C|GetCurrentSlowAmmo (Variables|Default|GetPlayer%20Ref%20Save)) (Variables|/Game/Blueprints/MainCharacter_BP.MainCharacter_BP_C|GetSlow%20Ammo%20Reserve (Variables|Default|GetPlayer%20Ref%20Save)) (Variables|/Game/Blueprints/MainCharacter_BP.MainCharacter_BP_C|GetRelicsCollect (Variables|Default|GetPlayer%20Ref%20Save))))
      (SaveGame|SaveGametoSlot (Variables|Default|GetSaveGameData) (Variables|Default|GetSaveSlot)))))

(fn LoadPlayerData
  (bind _returnvalue (SaveGame|DoesSaveGameExist (Variables|Default|GetSaveSlot)))
  (if _returnvalue
    (SaveGame|LoadGamefromSlot (Variables|Default|GetSaveSlot))
    (bind _asmain_character_bp (Utilities|Casting|CastToMainCharacter_BP (Game|GetPlayerCharacter 0)))
    (Variables|Default|SetPlayer%20Ref%20Load _asmain_character_bp)
    (bind _savegamedata (Variables|Default|GetSaveGameData)
      (:then
        (Utilities|FlowControl|Sequence
          (:then_0
            (Variables|/Game/Blueprints/MainCharacter_BP.MainCharacter_BP_C|SetHealth (Variables|Default|GetPlayer%20Ref%20Load) (.playerhealth (Variables|/Game/Blueprints/SaveSystem/SaveGameOcject.SaveGameOcject_C|GetPlayerSaveStruct _savegamedata))))
          (:then_1
            (Variables|/Game/Blueprints/MainCharacter_BP.MainCharacter_BP_C|SetCurrentStunAmmo (Variables|Default|GetPlayer%20Ref%20Load) (.stunammo (Variables|/Game/Blueprints/SaveSystem/SaveGameOcject.SaveGameOcject_C|GetPlayerSaveStruct _savegamedata)))
            (Variables|/Game/Blueprints/MainCharacter_BP.MainCharacter_BP_C|SetStun%20Ammo%20Reserve (Variables|Default|GetPlayer%20Ref%20Load) (.stunammoreserve (Variables|/Game/Blueprints/SaveSystem/SaveGameOcject.SaveGameOcject_C|GetPlayerSaveStruct _savegamedata))))
          (:then_2
            (Variables|/Game/Blueprints/MainCharacter_BP.MainCharacter_BP_C|SetCurrentSlowAmmo (Variables|Default|GetPlayer%20Ref%20Load) (.slowammor (Variables|/Game/Blueprints/SaveSystem/SaveGameOcject.SaveGameOcject_C|GetPlayerSaveStruct _savegamedata)))
            (Variables|/Game/Blueprints/MainCharacter_BP.MainCharacter_BP_C|SetSlow%20Ammo%20Reserve (Variables|Default|GetPlayer%20Ref%20Load) (.slowammoreserve (Variables|/Game/Blueprints/SaveSystem/SaveGameOcject.SaveGameOcject_C|GetPlayerSaveStruct _savegamedata))))
          (:then_3
            (Variables|/Game/Blueprints/MainCharacter_BP.MainCharacter_BP_C|SetRelicsCollect (Variables|Default|GetPlayer%20Ref%20Load) (.relicscollected (Variables|/Game/Blueprints/SaveSystem/SaveGameOcject.SaveGameOcject_C|GetPlayerSaveStruct _savegamedata))))))
      (:else))))

(fn ClearSaveData
  (SaveGame|DeleteGameinSlot (Variables|Default|GetSaveSlot)))