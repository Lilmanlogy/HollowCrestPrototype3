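; Health pickup actor that fully restores the player character's health and then destroys itself.
; A sphere overlap notifies MainCharacter_BP when it enters or leaves pickup range.
; The Pickup event calls PickedUp, which uses the player reference cached at BeginPlay.
; The pickup is consumed only when health is below maximum, so it stays in place at full health.
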(event OnComponentBeginOverlap(Sphere1)
  (params (OverlappedComponent :type Primitive%20Component%20Object%20Reference) (OtherActor :type Actor%20Object%20Reference) (OtherComp :type Primitive%20Component%20Object%20Reference) (OtherBodyIndex :type Integer) (bFromSweep :type Boolean) (SweepResult :type Hit%20Result%20Structure%20%28by%20ref%29))
  (bind _asmain_character_bp (Utilities|Casting|CastToMainCharacter_BP OtherActor))
  (Default|InPickupRange _asmain_character_bp))

(event OnComponentEndOverlap(Sphere1)
  (params (OverlappedComponent :type Primitive%20Component%20Object%20Reference) (OtherActor :type Actor%20Object%20Reference) (OtherComp :type Primitive%20Component%20Object%20Reference) (OtherBodyIndex :type Integer))
  (bind _asmain_character_bp (Utilities|Casting|CastToMainCharacter_BP OtherActor))
  (Default|OutPickupRange _asmain_character_bp))

(event Custom|PickedUp
  (bind _characterref (Variables|Default|GetCharacterRef))
  (bind _max_health (Variables|/Game/Blueprints/MainCharacter_BP.MainCharacter_BP_C|GetMax%20Health _characterref))
  (if (< (Variables|/Game/Blueprints/MainCharacter_BP.MainCharacter_BP_C|GetHealth _characterref) _max_health)
    (Variables|/Game/Blueprints/MainCharacter_BP.MainCharacter_BP_C|SetHealth _characterref _max_health)
    (Actor|DestroyActor)))

(event EventPickup
  (Utilities|Casting|CastToMainCharacter_BP (Game|GetPlayerCharacter 0))
  (CallFunction|PickedUp))

(event EventBeginPlay
  (bind _asmain_character_bp (Utilities|Casting|CastToMainCharacter_BP (Game|GetPlayerCharacter 0)))
  (Variables|Default|SetCharacterRef _asmain_character_bp))

(fn ConstructionScript)