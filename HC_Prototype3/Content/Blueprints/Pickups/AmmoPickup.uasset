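; Ammo pickup actor that adds to the player character's AmmoReserve and destroys itself when its Pickup event fires.
; Entering Sphere1 enables a throttled Tick that runs the character's line trace and compares the traced class to its own.
; A DoOnce shows the Pickup_Text widget on a match and resets when the widget is removed.
; Leaving the sphere hides the prompt but leaves Tick enabled.
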(event OnComponentBeginOverlap(Sphere1)
  (params (OverlappedComponent :type Primitive%20Component%20Object%20Reference) (OtherActor :type Actor%20Object%20Reference) (OtherComp :type Primitive%20Component%20Object%20Reference) (OtherBodyIndex :type Integer) (bFromSweep :type Boolean) (SweepResult :type Hit%20Result%20Structure%20%28by%20ref%29))
  (Utilities|Casting|CastToMainCharacter_BP OtherActor)
  (Actor|Tick|SetActorTickEnabled true))

(event OnComponentEndOverlap(Sphere1)
  (params (OverlappedComponent :type Primitive%20Component%20Object%20Reference) (OtherActor :type Actor%20Object%20Reference) (OtherComp :type Primitive%20Component%20Object%20Reference) (OtherBodyIndex :type Integer))
  (Utilities|Casting|CastToMainCharacter_BP OtherActor)
  (Utilities|FlowControl|Sequence
    (:then_0
      (if (UserInterface|Viewport|IsinViewport (Variables|Default|GetPickup%20Widget))
        (Widget|RemovefromParent (Variables|Default|GetPickup%20Widget))
        (Utilities|FlowControl|DoOnce false) ; enters at Reset
      ))
    (:then_1
      (Utilities|FlowControl|DoOnce false) ; enters at Reset
    )))

(event Custom|PickedUp
  (bind _characterref (Variables|Default|GetCharacterRef))
  (Variables|/Game/Blueprints/MainCharacter_BP.MainCharacter_BP_C|SetAmmo%20Reserve _characterref (+ (Variables|/Game/Blueprints/MainCharacter_BP.MainCharacter_BP_C|GetAmmo%20Reserve _characterref) 5))
  (Actor|DestroyActor))

(event EventTick
  (params (DeltaSeconds :type Float%20%28single-precision%29))
  (bind _characterref (Variables|Default|GetCharacterRef))
  (Default|LineTraceforObject _characterref)
  (if (== (Variables|/Game/Blueprints/MainCharacter_BP.MainCharacter_BP_C|GetTracedObejctClass _characterref) (Utilities|GetClass self))
    (Utilities|FlowControl|DoOnce false :!label _label
      (:Completed
        (UserInterface|Viewport|AddtoViewport (Variables|Default|GetPickup%20Widget) 0)))
    (elif (UserInterface|Viewport|IsinViewport (Variables|Default|GetPickup%20Widget))
      (Widget|RemovefromParent (Variables|Default|GetPickup%20Widget))
      (goto _label Reset))))

(event EventPickup
  (Utilities|Casting|CastToMainCharacter_BP (Game|GetPlayerCharacter 0))
  (CallFunction|PickedUp))

(event EventBeginPlay
  (bind _asmain_character_bp (Utilities|Casting|CastToMainCharacter_BP (Game|GetPlayerCharacter 0)))
  (Variables|Default|SetCharacterRef _asmain_character_bp)
  (Actor|Tick|SetActorTickEnabled false)
  (Actor|Tick|SetActorTickInterval 0.2)
  (bind _returnvalue (UserInterface|CreateWidget "/Game/Blueprints/Widgets/Pickup_Text.Pickup_Text_C"))
  (Variables|Default|SetPickup%20Widget _returnvalue))

(fn ConstructionScript)